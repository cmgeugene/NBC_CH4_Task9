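; BP_BnCGameState is the game state that runs the turn countdown for a turn-based, attempt-limited multiplayer game.
; OnSetTimer resets the remaining time and starts a looping timer that decrements it in small steps.
; At zero, the timer clears and fires a dispatcher for timeout handling, which messages every controller in BP_GM and deducts an attempt.
; StopTurnTimer cancels the countdown, such as at game end.
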(event `self.ReceiveBeginPlay`
  (bind _returnvalue (`self.GetTimerDuration`))
  (set `self.RemaningTimer` _returnvalue))

(event `OnSetTimer`
  ; 타이머 설정 시, 0.1초마다 시간 감소 이벤트 실행, 타이머 핸들 설정 후 이벤트 OnTimeOver() 구독
  (bind _returnvalue (`self.GetTimerDuration`))
  (set `self.RemaningTimer` _returnvalue)
  (bind _returnvalue_2 (`KismetSystemLibrary.K2_SetTimerDelegate` (`|CreateDelegate` :!event `DecrementTimer`) 0.1 true false 0.5))
  (add `self.OnTimerEnded` (`|CreateDelegate` :!event `OnTimerOver`))
  (set `self.TurnTimerHandle` _returnvalue_2))

(event `DecrementTimer`
  ; 시간 감소 로직 , 남은 시간 0이 되면 타이머 종료 후 이벤트 디스패처 호출
  (bind _output_get (set `self.RemaningTimer` (- (`self.RemaningTimer`) 0.1)))
  (if (<= _output_get 0.0)
    (`KismetSystemLibrary.K2_ClearAndInvalidateTimerHandle` (`self.TurnTimerHandle`))
    (`self.OnTimerEnded`)))

(event `OnTimerOver`
  ; 모든 플레이어에게 시간 초과 통보 후 기회 차감
  (bind _returnvalue (`GameplayStatics.GetActorOfClass` "/Game/Blueprints/BP_GM.BP_GM_C"))
  (for _array_element (`/Game/Blueprints/BP_GM.AllControllers` _returnvalue)
    (`/Game/Blueprints/BP_PlayerController.OnGotMessageFromServer` _array_element "Time Over!  The turn passes to the next player."))
  (`/Game/Blueprints/BP_GM.DeductAttempt` _returnvalue))

(event `StopTurnTimer`
  ; 현재 타이머 종료, 게임 종료 시 호출
  (`KismetSystemLibrary.K2_ClearAndInvalidateTimerHandle` (`self.TurnTimerHandle`)))

(fn `UserConstructionScript`)