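; Player controller that links the chat widget to BP_GM for multiplayer text chat.
; On BeginPlay it finds WBP_ChatUI after a short delay, binds its send event and assigns a random UserID, which OnLoginWithID can replace.
; Outgoing messages go to the game mode prefixed with the UserID, and messages returned from the server are added to the chat box.
; Enter focuses the chat and the mouse wheel scrolls it.
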(event `self.ReceiveBeginPlay`
  ;[1 0 0] BeginPlay()
  (if (not (`|EnumEquality` (`self.GetRemoteRole`) "ROLE_None"))
    (`KismetSystemLibrary.Delay` 0.2)
    (bind _foundwidgets (`WidgetBlueprintLibrary.GetAllWidgetsOfClass` "/Game/Blueprints/WBP_ChatUI.WBP_ChatUI_C"))
    (bind _output_get (set `self.ChatUIWidget` (`|GetArrayItem` _foundwidgets)))
    (bind _output_get_2 (set `self.WBP Chat Box` (`/Game/Blueprints/WBP_ChatUI.WBP_ChatBox` _output_get)))
    (add `/Game/Blueprints/WBP_ChatBox.SetMessageToUserController` _output_get_2 (`|CreateDelegate` :!event `OnSendMessageToServer`))
    ; 컨트롤러별 무작위 ID 할당
    (set `self.UserID` (`KismetStringLibrary.Conv_IntToString` (`KismetMathLibrary.RandomInteger` 50)))
    (`KismetSystemLibrary.PrintString` "random number allocated " true true (struct :`G` 0.66 :`B` 1.0 :`A` 1.0) 10.0)))

(event `Key|Enter`
  (params (Key :type "Key Structure"))
  ; 채팅창 조작 입력
  (:`Pressed`
    (`/Game/Blueprints/WBP_ChatBox.FocusChat` (`self.WBP Chat Box`))))

(event `OnSendMessageToServer`
  (params (Msg :type String))
  ; 위젯에서 채팅 입력했을 때 서버에 브로드캐스트 요청
  (bind _asbp_gm (cast `/Game/Blueprints/BP_GM` (`GameplayStatics.GetGameMode`)))
  (`/Game/Blueprints/BP_GM.OnGotMessageFromClient` _asbp_gm (`KismetStringLibrary.Concat_StrStr` (`self.UserID`) " : " Msg) self))

(event `Key|MouseScrollUp`
  (params (Key :type "Key Structure"))
  ; 채팅창 조작 입력
  (:`Pressed`
    (`/Game/Blueprints/WBP_ChatBox.Scroll` (`self.WBP Chat Box`) true)))

(event `Key|MouseScrollDown`
  (params (Key :type "Key Structure"))
  ; 채팅창 조작 입력
  (:`Pressed`
    (`/Game/Blueprints/WBP_ChatBox.Scroll` (`self.WBP Chat Box`) false)))

(event `OnGotMessageFromServer`
  (params (Message :type String))
  ; 서버->클라이언트 뿌려진 메세지 클라이언트의 채팅창에 출력
  (`/Game/Blueprints/WBP_ChatBox.AddChatMessage` (`self.WBP Chat Box`) Message))

(event `OnLoginWithID`
  (params (LoginID :type String))
  ; 유저 아이디 결정
  (set `self.UserID` LoginID))

(fn `OnRep_UserID`)

(fn `UserConstructionScript`)