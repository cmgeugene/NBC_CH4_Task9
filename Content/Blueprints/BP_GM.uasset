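; Game manager for a multiplayer Bulls and Cows number-guessing game played through chat on a listen server.
; It relays plain chat and routes slash messages to game start or guess validation and scoring.
; Turns rotate from a random player, skipping index 0 as the server and exhausted players, with the GameState running the timer.
; A correct guess scores a point; that or exhausted attempts ends the round with a scoreboard and reset.
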(event `GetRandomPlayerIndex`
  ; 선턴잡을 플레이어의 인덱스 랜덤 지정
  (set `self.TurnIndex` (`KismetMathLibrary.RandomIntegerInRange` 1 (- (`KismetArrayLibrary.Array_Length` (`self.AllPlayerStates`)) 1))))

(event `OnTurnEnded`
  ; 턴 종료시, 플레이어 입력 중지하고 인덱스 증가, 마지막 인덱스였으면 1로 초기화(서버 제외하기 위해) 그리고 다음턴 시작
  (set `BnCPlayerState.bCanInput` false (`|GetArrayItem` (`self.AllPlayerStates`) (`self.TurnIndex`)))
  (bind _result (`/Engine/EditorBlueprintResources/StandardMacros.IncrementInt` (`self.TurnIndex`))
    (:`  `
      (bind _output_get (set `self.TurnIndex` _result))
      (if (== _output_get (`KismetArrayLibrary.Array_Length` (`self.AllPlayerStates`)))
        (set `self.TurnIndex` 1))
      (`self.OnTurnStarted`))))

(event `OnTurnStarted`
  (bind _output (`|GetArrayItem` (`self.AllPlayerStates`) (`self.TurnIndex`)))
  (bind _output_2 (`|GetArrayItem` (`self.AllPlayerStates`) (`self.TurnIndex`)))
  ; 턴 시작 시, 전체 플레이어에게 턴 안내, 턴 인덱스에 해당하는 플레이어 입력 가능하도록 변경
  ;; 입력 기회 남아 있는지 검사
  (if (`BnCPlayerState.bHasNoChance` _output)
    (bind _asbp_player_controller (cast `/Game/Blueprints/BP_PlayerController` (`PlayerState.GetPlayerController` _output)))
    (for _array_element (`self.AllControllers`)
      (`/Game/Blueprints/BP_PlayerController.OnGotMessageFromServer` _array_element (`KismetStringLibrary.Concat_StrStr` (`/Game/Blueprints/BP_PlayerController.UserID` _asbp_player_controller) "'s turn. However, with no remaining attempts, the turn passes to the next player. \n")))
    (`self.OnTurnEnded`)
    (else
      (set `BnCPlayerState.bCanInput` true _output_2)
      (bind _asbp_player_controller_2 (cast `/Game/Blueprints/BP_PlayerController` (`PlayerState.GetPlayerController` _output_2)))
      (for _array_element_2 (`self.AllControllers`)
        (`/Game/Blueprints/BP_PlayerController.OnGotMessageFromServer` _array_element_2 (`KismetStringLibrary.Concat_StrStr` (`/Game/Blueprints/BP_PlayerController.UserID` _asbp_player_controller_2) "'s turn. Please submit guess. \n")))
      (`/Game/Blueprints/BP_BnCGameState.OnSetTimer` (`self.GameStateCache`)))))

(event `AddScoreToWinner`
  (bind _callerstate (`self.CallerState`))
  ; 정답자 점수 추가
  (bind _returnvalue (`BnCPlayerState.GetPlayerScore` _callerstate))
  (`BnCPlayerState.SetPlayerScore` _callerstate (+ _returnvalue 1)))

(event `OnGameStart`
  ; 게임 시작. 정답 생성하여 저장 후 모든 컨트롤러에게 시작 알림. 무작위 플레이어에게 선턴 부여.
  (bind _returnvalue (`NumberBaseball.GenerateSecretNumber`))
  (set `self.ANSWER` _returnvalue)
  (for _array_element (`self.AllControllers`)
    (`/Game/Blueprints/BP_PlayerController.OnGotMessageFromServer` _array_element " \n=== Bulls and Cows Game Start!! === \n")
    (`KismetSystemLibrary.Delay` 0.5)
    (`self.GetRandomPlayerIndex`)
    (`self.OnTurnStarted`)))

(event `OnGotCorrectAnswer`
  (params (CorrectAnswer :type String) (Caller :type String))
  ;[0 0.04872 1 0.5] 정답시 정답자 점수 추가 후 게임 종료 호출
  (`self.AddScoreToWinner`)
  (for _array_element (`self.AllControllers`)
    (`/Game/Blueprints/BP_PlayerController.OnGotMessageFromServer` _array_element (`KismetStringLibrary.Concat_StrStr` (`self.CallerID`) " submitted " (`KismetStringLibrary.Right` CorrectAnswer 3) ".. HOMERUN!!!! \n")))
  (`/Game/Blueprints/BP_BnCGameState.StopTurnTimer` (`self.GameStateCache`))
  (`KismetSystemLibrary.Delay` 2.0)
  (`self.OnGameEnded`))

(event `OnAnswerCommitted`
  (bind _callerid (`self.CallerID`))
  ; 올바른 입력이 들어왔을 때, 정답인지 틀린 답변인지
  (bind (_bulls _cows) (`NumberBaseball.SubmitGuess` (`self.PureMessage`) (`self.ANSWER`)))
  (if (and (== _bulls 3) (== _cows 0))
    ;;[0 0.04872 1 0.5] 정답
    (`self.OnGotCorrectAnswer` (`self.PureMessage`) _callerid)
    (else
      ;;[1 0 0 0.5] 오답
      (`self.OnGotWrongAnswer` _bulls _cows _callerid))))

(event `self.ReceiveBeginPlay`
  ;[0 0.15 0.008787 0.5] BeginPlay
  (`NumberBaseball.SetGameIsPlaying` false)
  ;; 모든 플레이어 컨트롤러, 스테이트 캐싱(충분한 delay가 없으면 다 안잡힘)
  (`KismetSystemLibrary.Delay` 3.0)
  (bind _outactors (`GameplayStatics.GetAllActorsOfClass` "/Game/Blueprints/BP_PlayerController.BP_PlayerController_C"))
  (set `self.AllControllers` _outactors)
  (bind _outactors_2 (`GameplayStatics.GetAllActorsOfClass` "/Game/Blueprints/BP_BnCPlayerState.BP_BnCPlayerState_C"))
  (set `self.AllPlayerStates` _outactors_2)
  (bind _returnvalue (`GameplayStatics.GetActorOfClass` "/Game/Blueprints/BP_BnCGameState.BP_BnCGameState_C"))
  (set `self.GameStateCache` _returnvalue))

(event `OnGotMessageFromClient`
  (params (Message :type String) (CalledController :type "/Game/Blueprints/BP_PlayerController Object Reference"))
  (`self.CacheQuerierContext` CalledController)
  (bind _output_get (set `self.Message` Message))
  ; 작성자 제외하고 입력 메세지만 추출 ( /123)
  (bind _output_get_2 (set `self.PureMessage` (`.RightS` (`KismetStringLibrary.Split` _output_get " : "))))
  ; 숫자 야구 명령어인지 확인
  (if (`KismetStringLibrary.EqualEqual_StrStr` (`KismetStringLibrary.Mid` _output_get_2 0 1) "/")
    ; 명령어라면 시작 명령어인지 확인
    (if (`KismetStringLibrary.EqualEqual_StrStr` (`self.PureMessage`) "/start")
      ;[0 0.15 0.008787 0.5] 게임 중인지 아닌지 확인 플래그
      (bind _returnvalue (`NumberBaseball.GetGameIsPlaying`))
      (if _returnvalue
        ; 이미 게임중입니다 출력
        (`/Game/Blueprints/BP_PlayerController.OnGotMessageFromServer` (`self.Caller`) "You are already in Playing.")
        (else
          ; 게임 중이 아니라면 게임 시작 호출
          (`self.OnGameStart`)
          ;;[0 0.15 0.02284 0.5] 게임 시작 플래그
          (`NumberBaseball.SetGameIsPlaying` true)))
      (else
        ; 올바른 형태의 명령어인가?
        (bind _returnvalue_2 (`NumberBaseball.IsValidGuess` (`self.PureMessage`)))
        (if _returnvalue_2
          ; 플레이어의 턴인지 아닌지 확인. 아니라면 입력불가
          (if (`BnCPlayerState.bCanInput` (`self.CallerState`))
            ; 입력 기회가 있는가, 없으면 입력 불가 출력
            (bind _returnvalue_3 (`BnCPlayerState.GetPlayerChance` (`self.CallerState`)))
            (if (>= _returnvalue_3 1)
              ; 올바른 명령어 입력 시
              (`self.OnAnswerCommitted`)
              (else
                (`/Game/Blueprints/BP_PlayerController.OnGotMessageFromServer` (`self.Caller`) "No attempts remaining. Input disabled.")))
            (else
              (`/Game/Blueprints/BP_PlayerController.OnGotMessageFromServer` (`self.Caller`) " \nIt's not your turn. \nPlease wait for other player's answer.")))
          (else
            ; 잘못된 명령어 입력 시
            (`/Game/Blueprints/BP_PlayerController.OnGotMessageFromServer` (`self.Caller`) "Invalid Input. Please input valid Command. \n")))))
    (else
      ; 클라이언트 -> 서버 일반 채팅 처리
      (for _array_element (`self.AllControllers`)
        (`/Game/Blueprints/BP_PlayerController.OnGotMessageFromServer` _array_element (`self.Message`))))))

(event `DeductAttempt`
  (bind _output (`|GetArrayItem` (`self.AllPlayerStates`) (`self.TurnIndex`)))
  (bind _output_2 (`|GetArrayItem` (`self.AllPlayerStates`) (`self.TurnIndex`)))
  ;[0.15 0.1348 0 0.5] 도전 기회 차감, 0되면 입력 불가 상태로 변경
  (`|ExecutionSequence`
    (:`then_0`
      ;; 현재 턴인 플레이어 기회 차감
      (bind _returnvalue (`BnCPlayerState.GetPlayerChance` _output_2))
      (`BnCPlayerState.SetPlayerChance` _output_2 (- _returnvalue 1))
      (bind _asbp_player_controller (cast `/Game/Blueprints/BP_PlayerController` (`PlayerState.GetPlayerController` _output_2)))
      ;; 모든 플레이어에게 차감 통지
      (for _array_element (`self.AllControllers`)
        (bind _returnvalue_2 (`BnCPlayerState.GetPlayerChance` _output_2))
        (`/Game/Blueprints/BP_PlayerController.OnGotMessageFromServer` _array_element (`KismetTextLibrary.Conv_TextToString` (`|FormatText` " \n{user id} has {remainattempts} left now. \n" (`/Game/Blueprints/BP_PlayerController.UserID` _asbp_player_controller) _returnvalue_2)))))
    (:`then_1`
      ;; 현재 플레이어에게 남은 기회가 없다면 기회 없음 플래그 활성화 후 무승부 카운터 증가
      (bind _returnvalue_3 (`BnCPlayerState.GetPlayerChance` _output))
      (if (<= _returnvalue_3 0)
        (set `BnCPlayerState.bCanInput` false _output)
        (set `BnCPlayerState.bHasNoChance` true _output)
        (set `self.AmountOfNoChance` (+ (`self.AmountOfNoChance`) 1))
        (bind _asbp_player_controller_2 (cast `/Game/Blueprints/BP_PlayerController` (`PlayerState.GetPlayerController` (`|GetArrayItem` (`self.AllPlayerStates`) (`self.TurnIndex`)))))
        (`/Game/Blueprints/BP_PlayerController.OnGotMessageFromServer` _asbp_player_controller_2 "No attempts remaining. Input disabled.")))
    (:`then_2`
      ;; 기회 소진 플레이어 수 확인
      (bind _bisdrawgame (`self.IsDrawGame` (`KismetArrayLibrary.Array_Length` (`self.AllControllers`)) (`self.AmountOfNoChance`)))
      (if _bisdrawgame
        ;; 무승부 통지 -> 턴 타이머 종료 -> 게임 종료
        (for _array_element_2 (`self.AllControllers`)
          (`/Game/Blueprints/BP_PlayerController.OnGotMessageFromServer` _array_element_2 " \nAll Players have 0 attemps. DRAW GAME !! \n")
          (`/Game/Blueprints/BP_BnCGameState.StopTurnTimer` (`self.GameStateCache`)))
        (`KismetSystemLibrary.Delay` 2.0)
        (`self.OnGameEnded`)
        (else
          ;; 게임 속행
          (`self.OnTurnEnded`))))))

(event `OnGotWrongAnswer`
  (params (Bulls :type Integer) (Cows :type Integer) (CallerID :type String))
  ;[1 0 0 0.5] 오답일 때, 아웃인지 일부 정답인지 출력 후 도전 기회 차감
  (for _array_element (`self.AllControllers`)
    (if (and (== Bulls 0) (== Cows 0))
      (`/Game/Blueprints/BP_PlayerController.OnGotMessageFromServer` _array_element (`KismetStringLibrary.Concat_StrStr` CallerID " submitted " (`KismetStringLibrary.Right` (`self.PureMessage`) 3) ". OUT!!"))
      (else
        (`/Game/Blueprints/BP_PlayerController.OnGotMessageFromServer` _array_element (`KismetStringLibrary.Concat_StrStr` CallerID " submitted " (`KismetStringLibrary.Right` (`self.PureMessage`) 3) (`KismetTextLibrary.Conv_TextToString` (`|FormatText` ". {S} S {B} B !" Bulls Cows)))))))
  (`self.DeductAttempt`))

(event `CacheQuerierContext`
  (params (Querier :type "/Game/Blueprints/BP_PlayerController Object Reference"))
  ;[0 0.1379 0.15 0.5] 요청 발신자 캐싱
  (bind _output_get (set `self.Caller` Querier))
  (set `self.CallerID` (`/Game/Blueprints/BP_PlayerController.UserID` _output_get))
  (bind _asbp_bn_cplayer_state (cast `/Game/Blueprints/BP_BnCPlayerState` (`Controller.PlayerState` _output_get)))
  (set `self.CallerState` _asbp_bn_cplayer_state))

(event `OnGameEnded`
  ; 게임 종료 시
  (`NumberBaseball.SetGameIsPlaying` false)
  (for _array_element (`self.AllControllers`)
    (`|ExecutionSequence`
      (:`then_0`
        (`/Game/Blueprints/BP_PlayerController.OnGotMessageFromServer` _array_element "======= Game Ended  ======= \n")
        (`/Game/Blueprints/BP_PlayerController.OnGotMessageFromServer` _array_element "[ Score Board ]"))
      (:`then_1`
        ;; 모든 플레이어 컨트롤러, 스테이트에서 UserID와 Score 가져와 출력
        (for _array_element_2 (`self.AllPlayerStates`)
          (bind _asbp_player_controller (cast `/Game/Blueprints/BP_PlayerController` (`PlayerState.GetPlayerController` _array_element_2)))
          (bind _userid (`/Game/Blueprints/BP_PlayerController.UserID` _asbp_player_controller))
          ;;; 서버 (리슨 서버) 점수는 제외
          (if (not (`KismetStringLibrary.EqualEqual_StrStr` _userid "Server"))
            (bind _returnvalue (`BnCPlayerState.GetPlayerScore` _array_element_2))
            (bind _output_get (set `self.GameResult` (`KismetStringLibrary.Concat_StrStr` _userid " got " (`KismetStringLibrary.Conv_IntToString` _returnvalue) "" "pt.")))
            (`/Game/Blueprints/BP_PlayerController.OnGotMessageFromServer` _array_element _output_get)))
        (`/Game/Blueprints/BP_PlayerController.OnGotMessageFromServer` _array_element " \nType '/start' to play again! \n"))))
  ;; 점수 외 변수 초기화
  (for _array_element_3 (`self.AllPlayerStates`)
    (`BnCPlayerState.SetPlayerChance` _array_element_3 3)
    (set `BnCPlayerState.bCanInput` false _array_element_3)
    (set `BnCPlayerState.bHasNoChance` false _array_element_3))
  (set `self.AmountOfNoChance` 0))

(fn `IsDrawGame`
  (params (Controller_num :type Integer) (AmountOfNoChance :type Integer))
  (returns (bIsDrawGame :type Boolean))
  (if (== (- Controller_num 1) AmountOfNoChance)
    (return true)
    (else
      (return false))))

(fn `UserConstructionScript`)